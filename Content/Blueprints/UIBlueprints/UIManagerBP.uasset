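; UIManagerBP is an actor that manages the in-game options menu.
; On BeginPlay it enables input from the first player controller and creates an OptionUIBP widget once, keeping it for reuse.
; Pressing Tab alternates through a FlipFlop: it adds the widget to the viewport, pauses the game and shows the mouse cursor, then reverses all three on the next press.
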(event EventBeginPlay
  (Utilities|FlowControl|Sequence
    (:then_0
      ;[1 1 1] 인풋 허용
      (Input|EnableInput (Game|GetPlayerController 0)))
    (:then_1
      ;[1 1 1] OptionUI생성
      (bind _returnvalue (UserInterface|CreateWidget "/Game/Blueprints/UIBlueprints/OptionUIBP.OptionUIBP_C"))
      (Variables|Default|SetOptionUI _returnvalue))))

(event Input|KeyboardEvents|Tab
  (params (Key :type Key%20Structure :default "None"))
  (bind _returnvalue (Game|GetPlayerController 0))
  (bind _optionui (Variables|Default|GetOptionUI))
  ;[1 1 1] Option창 진입/탈출 로직
  (:Pressed
    (Utilities|FlowControl|FlipFlop
      (:A
        (UserInterface|Viewport|AddtoViewport _optionui 0)
        (Game|SetGamePaused true)
        (Variables|/Script/Engine.PlayerController|SetbShowMouseCursor _returnvalue true))
      (:B
        (Widget|RemovefromParent _optionui)
        (Game|SetGamePaused false)
        (Variables|/Script/Engine.PlayerController|SetbShowMouseCursor _returnvalue false)))))

(fn ConstructionScript)